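; Smart building manager that turns mouse clicks on buildings into floor layering and pull/push displays.
; At BeginPlay it maps every BP_SMBD_Building by name; a click without drag traces from the camera and parses the hit actor's last "Building:Floor" tag.
; If the building is idle, roof or top-floor hits toggle layering, while other floors hide all buildings' area actors and pull or push that floor.
; Disconnected FlipFlop chains hold API tests.
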(event EventBeginPlay
  ;[0 0 0] BeginPlay
  (bind _outactors (Actor|GetAllActorsOfClass "/Game/AssetLibrary/4_BPTools/SmartBuilding/BP/BP_SMBD_Building.BP_SMBD_Building_C"))
  (for _array_element _outactors
    (Utilities|Map|Add (Variables|Default|GetAll_SMBD) (CallFunction|DisplayNameCutNubmer (Utilities|GetDisplayName (Variables|/Game/AssetLibrary/4_BPTools/SmartBuilding/BP/BP_SMBD_Building.BP_SMBD_Building_C|GetBuildingActor _array_element))) _array_element)))

(event Input|MouseEvents|LeftMouseButton
  (params (Key :type Key%20Structure))
  (bind _returnvalue (Game|GetPlayerController 0))
  (bind _returnvalue_2 (Game|GetPlayerCameraManager 0))
  (bind _openclick_ (Variables|Default|GetOpenClick?))
  (bind (_locationx _locationy) (Game|Player|GetMousePosition _returnvalue))
  (bind _transformcomponent (Variables|/Script/Engine.PlayerCameraManager|GetTransformComponent _returnvalue_2))
  (bind _returnvalue_3 (Transformation|GetWorldLocation _transformcomponent))
  ;[0 0 0] LineTrace
  (:Pressed
    (if _openclick_
      (Variables|Default|SetLocation_MousePressed (Math|Vector|MakeVector _locationx _locationy 0.0))))
  (:Released
    (if _openclick_
      (Utilities|FlowControl|Sequence
        (:then_0
          (Variables|Default|SetLocation_MouseReleased (Math|Vector|MakeVector _locationx _locationy 0.0)))
        (:then_1
          (if (Math|Vector|Equal(Vector) (Variables|Default|GetLocation_MousePressed) (Variables|Default|GetLocation_MouseReleased) 0.0001)
            (bind _outhit (Collision|LineTraceByChannel _returnvalue_3 (+ _returnvalue_3 (* (.WorldDirection (Game|Player|ConvertMouseLocationToWorldSpace (Game|GetPlayerController 0))) (Variables|Default|GetTraceLineLength))) "TraceTypeQuery1" true 0 "None" true "(R=1.000000,G=0.000000,B=0.000000,A=1.000000)" "(R=0.000000,G=1.000000,B=0.000000,A=1.000000)" 6e+01))
            (if (.bBlockingHit (Collision|BreakHitResult _outhit))
              (if (Actor|ActorHasTag (.HitActor (Collision|BreakHitResult _outhit)) "SMBD")
                (Development|PrintString (Utilities|String|GetSubstring (Utilities|String|ToString(Name) (Utilities|Array|Get(acopy) (Variables|/Script/Engine.Actor|GetTags (.HitActor (Collision|BreakHitResult _outhit))) (- (Utilities|Array|Length (Variables|/Script/Engine.Actor|GetTags (.HitActor (Collision|BreakHitResult _outhit)))) 1))) 0 (Utilities|String|FindSubstring (Utilities|String|ToString(Name) (Utilities|Array|Get(acopy) (Variables|/Script/Engine.Actor|GetTags (.HitActor (Collision|BreakHitResult _outhit))) (- (Utilities|Array|Length (Variables|/Script/Engine.Actor|GetTags (.HitActor (Collision|BreakHitResult _outhit)))) 1))) ":")) false false)
                (Variables|Default|SetNow (.Value (Utilities|Map|Find (Variables|Default|GetAll_SMBD) (Utilities|String|GetSubstring (Utilities|String|ToString(Name) (Utilities|Array|Get(acopy) (Variables|/Script/Engine.Actor|GetTags (.HitActor (Collision|BreakHitResult _outhit))) (- (Utilities|Array|Length (Variables|/Script/Engine.Actor|GetTags (.HitActor (Collision|BreakHitResult _outhit)))) 1))) 0 (Utilities|String|FindSubstring (Utilities|String|ToString(Name) (Utilities|Array|Get(acopy) (Variables|/Script/Engine.Actor|GetTags (.HitActor (Collision|BreakHitResult _outhit))) (- (Utilities|Array|Length (Variables|/Script/Engine.Actor|GetTags (.HitActor (Collision|BreakHitResult _outhit)))) 1))) ":")))))
                (Utilities|IsValid (Variables|Default|GetNow)
                  (:Is%20Valid
                    (if (not (Variables|/Game/AssetLibrary/4_BPTools/SmartBuilding/BP/BP_SMBD_Building.BP_SMBD_Building_C|GetIsRun? (Variables|Default|GetNow)))
                      (if (or (Utilities|Name|Equal(Name) (Utilities|String|StringToName (Utilities|String|GetSubstring (Utilities|String|ToString(Name) (Utilities|Array|Get(acopy) (Variables|/Script/Engine.Actor|GetTags (.HitActor (Collision|BreakHitResult _outhit))) (- (Utilities|Array|Length (Variables|/Script/Engine.Actor|GetTags (.HitActor (Collision|BreakHitResult _outhit)))) 1))) (+ (Utilities|String|FindSubstring (Utilities|String|ToString(Name) (Utilities|Array|Get(acopy) (Variables|/Script/Engine.Actor|GetTags (.HitActor (Collision|BreakHitResult _outhit))) (- (Utilities|Array|Length (Variables|/Script/Engine.Actor|GetTags (.HitActor (Collision|BreakHitResult _outhit)))) 1))) ":") 1) (Utilities|String|Len (Utilities|String|ToString(Name) (Utilities|Array|Get(acopy) (Variables|/Script/Engine.Actor|GetTags (.HitActor (Collision|BreakHitResult _outhit))) (- (Utilities|Array|Length (Variables|/Script/Engine.Actor|GetTags (.HitActor (Collision|BreakHitResult _outhit)))) 1)))))) "Roof") (Utilities|Name|Equal(Name) (Utilities|String|StringToName (Utilities|String|GetSubstring (Utilities|String|ToString(Name) (Utilities|Array|Get(acopy) (Variables|/Script/Engine.Actor|GetTags (.HitActor (Collision|BreakHitResult _outhit))) (- (Utilities|Array|Length (Variables|/Script/Engine.Actor|GetTags (.HitActor (Collision|BreakHitResult _outhit)))) 1))) (+ (Utilities|String|FindSubstring (Utilities|String|ToString(Name) (Utilities|Array|Get(acopy) (Variables|/Script/Engine.Actor|GetTags (.HitActor (Collision|BreakHitResult _outhit))) (- (Utilities|Array|Length (Variables|/Script/Engine.Actor|GetTags (.HitActor (Collision|BreakHitResult _outhit)))) 1))) ":") 1) (Utilities|String|Len (Utilities|String|ToString(Name) (Utilities|Array|Get(acopy) (Variables|/Script/Engine.Actor|GetTags (.HitActor (Collision|BreakHitResult _outhit))) (- (Utilities|Array|Length (Variables|/Script/Engine.Actor|GetTags (.HitActor (Collision|BreakHitResult _outhit)))) 1)))))) (Utilities|String|StringToName (Utilities|String|Append (Utilities|String|ToString(Integer) (Variables|/Game/AssetLibrary/4_BPTools/SmartBuilding/BP/BP_SMBD_Building.BP_SMBD_Building_C|GetTopFloor (Variables|Default|GetNow))) "F"))))
                        (if (Variables|/Game/AssetLibrary/4_BPTools/SmartBuilding/BP/BP_SMBD_Building.BP_SMBD_Building_C|GetisBuildingLayering? (Variables|Default|GetNow))
                          (Utilities|IsValid (Variables|Default|GetNow)
                            (:Is%20Valid
                              (Default|APISMBDFloorBacktoNormalDisplay (Variables|Default|GetNow))))
                          (else
                            (Utilities|IsValid (Variables|Default|GetNow)
                              (:Is%20Valid
                                (Default|APISMBDFloorLayeringDisplay (Variables|Default|GetNow))))))
                        (else
                          (bind _keys (Utilities|Map|Keys (Variables|/Game/AssetLibrary/4_BPTools/SmartBuilding/BP/BP_SMBD_Building.BP_SMBD_Building_C|GetBuilding_Floor (Variables|Default|GetNow))))
                          (bind _values (Utilities|Map|Values (Variables|Default|GetAll_SMBD)))
                          (for _array_element _values
                            (bind _asbp_smbd_building (Utilities|Casting|CastToBP_SMBD_Building _array_element))
                            (Default|HidetAllAreaActor _asbp_smbd_building))
                          (if (Utilities|Enum|Equal(Enum) (Utilities|Array|Get(acopy) (Variables|/Game/AssetLibrary/4_BPTools/SmartBuilding/BP/BP_SMBD_Building.BP_SMBD_Building_C|GetBuilding_LayeringState (Variables|Default|GetNow)) (Utilities|Array|FindItem _keys (Utilities|String|ToString(Name) (Utilities|String|StringToName (Utilities|String|GetSubstring (Utilities|String|ToString(Name) (Utilities|Array|Get(acopy) (Variables|/Script/Engine.Actor|GetTags (.HitActor (Collision|BreakHitResult _outhit))) (- (Utilities|Array|Length (Variables|/Script/Engine.Actor|GetTags (.HitActor (Collision|BreakHitResult _outhit)))) 1))) (+ (Utilities|String|FindSubstring (Utilities|String|ToString(Name) (Utilities|Array|Get(acopy) (Variables|/Script/Engine.Actor|GetTags (.HitActor (Collision|BreakHitResult _outhit))) (- (Utilities|Array|Length (Variables|/Script/Engine.Actor|GetTags (.HitActor (Collision|BreakHitResult _outhit)))) 1))) ":") 1) (Utilities|String|Len (Utilities|String|ToString(Name) (Utilities|Array|Get(acopy) (Variables|/Script/Engine.Actor|GetTags (.HitActor (Collision|BreakHitResult _outhit))) (- (Utilities|Array|Length (Variables|/Script/Engine.Actor|GetTags (.HitActor (Collision|BreakHitResult _outhit)))) 1))))))))) "0")
                            (Utilities|IsValid (Variables|Default|GetNow)
                              (:Is%20Valid
                                (Default|APISMBDFloorPull (Variables|Default|GetNow) (Math|Conversions|ToInteger(Byte) (Utilities|String|ToString(Name) (Utilities|String|StringToName (Utilities|String|GetSubstring (Utilities|String|ToString(Name) (Utilities|Array|Get(acopy) (Variables|/Script/Engine.Actor|GetTags (.HitActor (Collision|BreakHitResult _outhit))) (- (Utilities|Array|Length (Variables|/Script/Engine.Actor|GetTags (.HitActor (Collision|BreakHitResult _outhit)))) 1))) (+ (Utilities|String|FindSubstring (Utilities|String|ToString(Name) (Utilities|Array|Get(acopy) (Variables|/Script/Engine.Actor|GetTags (.HitActor (Collision|BreakHitResult _outhit))) (- (Utilities|Array|Length (Variables|/Script/Engine.Actor|GetTags (.HitActor (Collision|BreakHitResult _outhit)))) 1))) ":") 1) (Utilities|String|Len (Utilities|String|ToString(Name) (Utilities|Array|Get(acopy) (Variables|/Script/Engine.Actor|GetTags (.HitActor (Collision|BreakHitResult _outhit))) (- (Utilities|Array|Length (Variables|/Script/Engine.Actor|GetTags (.HitActor (Collision|BreakHitResult _outhit)))) 1)))))))))))
                            (elif (Utilities|Enum|Equal(Enum) (Utilities|Array|Get(acopy) (Variables|/Game/AssetLibrary/4_BPTools/SmartBuilding/BP/BP_SMBD_Building.BP_SMBD_Building_C|GetBuilding_LayeringState (Variables|Default|GetNow)) (Utilities|Array|FindItem _keys (Utilities|String|ToString(Name) (Utilities|String|StringToName (Utilities|String|GetSubstring (Utilities|String|ToString(Name) (Utilities|Array|Get(acopy) (Variables|/Script/Engine.Actor|GetTags (.HitActor (Collision|BreakHitResult _outhit))) (- (Utilities|Array|Length (Variables|/Script/Engine.Actor|GetTags (.HitActor (Collision|BreakHitResult _outhit)))) 1))) (+ (Utilities|String|FindSubstring (Utilities|String|ToString(Name) (Utilities|Array|Get(acopy) (Variables|/Script/Engine.Actor|GetTags (.HitActor (Collision|BreakHitResult _outhit))) (- (Utilities|Array|Length (Variables|/Script/Engine.Actor|GetTags (.HitActor (Collision|BreakHitResult _outhit)))) 1))) ":") 1) (Utilities|String|Len (Utilities|String|ToString(Name) (Utilities|Array|Get(acopy) (Variables|/Script/Engine.Actor|GetTags (.HitActor (Collision|BreakHitResult _outhit))) (- (Utilities|Array|Length (Variables|/Script/Engine.Actor|GetTags (.HitActor (Collision|BreakHitResult _outhit)))) 1))))))))) "1")
                              (Utilities|IsValid (Variables|Default|GetNow)
                                (:Is%20Valid
                                  (Default|APISMBDFloorPush (Variables|Default|GetNow) (Math|Conversions|ToInteger(Byte) (Utilities|String|ToString(Name) (Utilities|String|StringToName (Utilities|String|GetSubstring (Utilities|String|ToString(Name) (Utilities|Array|Get(acopy) (Variables|/Script/Engine.Actor|GetTags (.HitActor (Collision|BreakHitResult _outhit))) (- (Utilities|Array|Length (Variables|/Script/Engine.Actor|GetTags (.HitActor (Collision|BreakHitResult _outhit)))) 1))) (+ (Utilities|String|FindSubstring (Utilities|String|ToString(Name) (Utilities|Array|Get(acopy) (Variables|/Script/Engine.Actor|GetTags (.HitActor (Collision|BreakHitResult _outhit))) (- (Utilities|Array|Length (Variables|/Script/Engine.Actor|GetTags (.HitActor (Collision|BreakHitResult _outhit)))) 1))) ":") 1) (Utilities|String|Len (Utilities|String|ToString(Name) (Utilities|Array|Get(acopy) (Variables|/Script/Engine.Actor|GetTags (.HitActor (Collision|BreakHitResult _outhit))) (- (Utilities|Array|Length (Variables|/Script/Engine.Actor|GetTags (.HitActor (Collision|BreakHitResult _outhit)))) 1))))))))))))))))))))))))))

(event Input|KeyboardEvents|F
  (params (Key :type Key%20Structure))
  ;[0 0 0] Anykey
)

(event Input|KeyboardEvents|4
  (params (Key :type Key%20Structure))
  ;[0 0 0] Anykey
)

(event Input|KeyboardEvents|1
  (params (Key :type Key%20Structure))
  ;[0 0 0] Anykey
)

(event Input|KeyboardEvents|2
  (params (Key :type Key%20Structure))
  ;[0 0 0] Anykey
)

(event Input|KeyboardEvents|3
  (params (Key :type Key%20Structure))
  ;[0 0 0] Anykey
)

(fn ConstructionScript)