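; Smart-building controller that animates a building's floors into an exploded vertical stack and slides single floors out and back.
; Parse_FloorActor maps attached actors to floors and area meshes by name (root component or display name), and BeginPlay tags floors and their descendants.
; API functions drive timeline-lerped layering and pull/push, gated by busy and per-floor state.
; Visibility uses zero scale, while pulling fades areas in through a material parameter collection.
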(event Custom|Parse_FloorActor
  (bind _buildingactor (Variables|Default|GetBuildingActor))
  (bind _outactors (Actor|GetAttachedActors _buildingactor true false))
  (bind _returnvalue (Utilities|Array|Length _outactors))
  ;[0 0 0] Parse_FloorActor
  (Utilities|Map|Clear (Variables|Default|GetAreaActors))
  (Utilities|Map|Clear (Variables|Default|GetBuilding_Floor))
  (Utilities|FlowControl|Sequence
    (:then_0
      (goto _label Reset))
    (:then_1
      (bind _counter (Utilities|FlowControl|DoN (select (< (Variables|Default|GetLowestFloor) 0) _returnvalue (+ _returnvalue 1)) :!label _label)
        (:Exit
          (for _array_element _outactors
            (if (Utilities|Enum|Equal(Enum) (Utilities|Select :Index (Variables|Default|GetE_FloorBuildType) :NewEnumerator0 (Utilities|GetObjectName (Variables|/Script/Engine.Actor|GetRootComponent _array_element)) :NewEnumerator1 (CallFunction|DisplayNameCutNubmer (Utilities|GetDisplayName _array_element))) (Utilities|String|Append (Utilities|String|ToString(Integer) (+ (Variables|Default|GetLowestFloor) (- _counter 1))) "F"))
              (Utilities|Map|Add (Variables|Default|GetBuilding_Floor) (Utilities|String|Append (Utilities|String|ToString(Integer) (+ (Variables|Default|GetLowestFloor) (- _counter 1))) "F") _array_element)
              (elif (Utilities|Enum|Equal(Enum) (Utilities|Select :Index (Variables|Default|GetE_FloorBuildType) :NewEnumerator0 (Utilities|GetObjectName (Variables|/Script/Engine.Actor|GetRootComponent _array_element)) :NewEnumerator1 (CallFunction|DisplayNameCutNubmer (Utilities|GetDisplayName _array_element))) "Roof")
                (if (not (.ReturnValue (Utilities|Map|Find (Variables|Default|GetBuilding_Floor) "Roof")))
                  (Utilities|Map|Add (Variables|Default|GetBuilding_Floor) "Roof" _array_element)))))
          (goto _label))))
    (:then_2
      (CallFunction|GetAreaActor))))

(event Custom|ResetLayering
  (params (Dimension%201 :type Integer))
  (bind _building_floor (Variables|Default|GetBuilding_Floor))
  ;[0 0 0] Building_BackToNormal
  (bind _values (Utilities|Map|Values _building_floor))
  (bind _keys (Utilities|Map|Keys _building_floor))
  (Transformation|SetActorLocation (Utilities|Array|Get(acopy) _values Dimension%201) (Math|Vector|MakeVector (.x (.Value (Utilities|Map|Find (Variables|Default|GetFloorLocation_PullPush) (Utilities|Array|Get(acopy) _keys Dimension%201)))) (.y (.Value (Utilities|Map|Find (Variables|Default|GetFloorLocation_PullPush) (Utilities|Array|Get(acopy) _keys Dimension%201)))) (.z (Transformation|GetActorLocation (.Value (Utilities|Map|Find (Variables|Default|GetBuilding_Floor) (Utilities|Array|Get(acopy) _keys Dimension%201)))))) false false)
  (Utilities|Array|SetArrayElem (Variables|Default|GetBuilding_LayeringState) Dimension%201 "0"))

(event Custom|SMBD_FloorPush
  (params (NumberOfFloor :type Integer))
  (bind _returnvalue (Utilities|String|ToString(Integer) NumberOfFloor))
  (bind _returnvalue_2 (Utilities|String|Append _returnvalue "F"))
  ;[0 0 0] Building_Push
  (if (not (Variables|Default|GetIsRun?))
    (if (Variables|Default|GetisBuildingLayering?)
      (bind _keys (Utilities|Map|Keys (Variables|Default|GetBuilding_Floor)))
      (Variables|Default|SetNow_FloorNumber (Utilities|Array|FindItem _keys _returnvalue_2))
      (Variables|Default|SetNow_FloorName _returnvalue_2)
      (if (Utilities|Enum|Equal(Enum) (Utilities|Array|Get(acopy) (Variables|Default|GetBuilding_LayeringState) (Variables|Default|GetNow_FloorNumber)) "1")
        (Variables|Default|SetIsRun? true)
        (Utilities|FlowControl|Sequence
          (:then_1
            (bind _新建轨迹_0 (Timeline|时间轴_3 PlayFromStart)
              (:Update
                (Utilities|IsValid (.Value (Utilities|Map|Find (Variables|Default|GetBuilding_Floor) (Variables|Default|GetNow_FloorName)))
                  (:Is%20Valid
                    (Transformation|SetActorLocation (.Value (Utilities|Map|Find (Variables|Default|GetBuilding_Floor) (Variables|Default|GetNow_FloorName))) (Math|Vector|MakeVector (.x (Math|Vector|Lerp(Vector) (+ (.Value (Utilities|Map|Find (Variables|Default|GetFloorLocation_PullPush) (Variables|Default|GetNow_FloorName))) (Variables|Default|GetFloorPull_Dir)) (.Value (Utilities|Map|Find (Variables|Default|GetFloorLocation_PullPush) (Variables|Default|GetNow_FloorName))) _新建轨迹_0)) (.y (Math|Vector|Lerp(Vector) (+ (.Value (Utilities|Map|Find (Variables|Default|GetFloorLocation_PullPush) (Variables|Default|GetNow_FloorName))) (Variables|Default|GetFloorPull_Dir)) (.Value (Utilities|Map|Find (Variables|Default|GetFloorLocation_PullPush) (Variables|Default|GetNow_FloorName))) _新建轨迹_0)) (.Z (Math|Vector|BreakVector (Transformation|GetActorLocation (.Value (Utilities|Map|Find (Variables|Default|GetBuilding_Floor) (Variables|Default|GetNow_FloorName))))))) false false))))
              (:Finished
                (Variables|Default|SetIsRun? false)
                (Utilities|Array|SetArrayElem (Variables|Default|GetBuilding_LayeringState) (Variables|Default|GetNow_FloorNumber) "0"))))
          (:then_2
            (CallFunction|HideAreaActor _returnvalue_2)))))))

(event Custom|SMBD_FloorPull
  (params (NumberOfFloor :type Integer))
  (bind _returnvalue (Utilities|String|ToString(Integer) NumberOfFloor))
  (bind _returnvalue_2 (Utilities|String|Append _returnvalue "F"))
  ;[0 0 0] Building_Pull
  (if (not (Variables|Default|GetIsRun?))
    (if (Variables|Default|GetisBuildingLayering?)
      (bind _keys (Utilities|Map|Keys (Variables|Default|GetBuilding_Floor)))
      (Variables|Default|SetNow_FloorNumber (Utilities|Array|FindItem _keys _returnvalue_2))
      (Variables|Default|SetNow_FloorName _returnvalue_2)
      (if (Utilities|Enum|Equal(Enum) (Utilities|Array|Get(acopy) (Variables|Default|GetBuilding_LayeringState) (Variables|Default|GetNow_FloorNumber)) "0")
        (Variables|Default|SetIsRun? true)
        (Utilities|FlowControl|Sequence
          (:then_0
            (bind _新建轨迹_0 (Timeline|时间轴_2 PlayFromStart)
              (:Update
                (Utilities|IsValid (.Value (Utilities|Map|Find (Variables|Default|GetBuilding_Floor) (Variables|Default|GetNow_FloorName)))
                  (:Is%20Valid
                    (Transformation|SetActorLocation (.Value (Utilities|Map|Find (Variables|Default|GetBuilding_Floor) (Variables|Default|GetNow_FloorName))) (Math|Vector|MakeVector (.x (Math|Vector|Lerp(Vector) (.Value (Utilities|Map|Find (Variables|Default|GetFloorLocation_PullPush) (Variables|Default|GetNow_FloorName))) (+ (.Value (Utilities|Map|Find (Variables|Default|GetFloorLocation_PullPush) (Variables|Default|GetNow_FloorName))) (Variables|Default|GetFloorPull_Dir)) _新建轨迹_0)) (.y (Math|Vector|Lerp(Vector) (.Value (Utilities|Map|Find (Variables|Default|GetFloorLocation_PullPush) (Variables|Default|GetNow_FloorName))) (+ (.Value (Utilities|Map|Find (Variables|Default|GetFloorLocation_PullPush) (Variables|Default|GetNow_FloorName))) (Variables|Default|GetFloorPull_Dir)) _新建轨迹_0)) (.Z (Math|Vector|BreakVector (Transformation|GetActorLocation (.Value (Utilities|Map|Find (Variables|Default|GetBuilding_Floor) (Variables|Default|GetNow_FloorName))))))) false false)
                    (Rendering|Material|SetScalarParameterValue "/Game/AssetLibrary/4_BPTools/SmartBuilding/Materials/MPC_Area.MPC_Area" "Area_Opacity" (Math|Float|Lerp 0.0 1.0 _新建轨迹_0) :!class /Script/Engine.KismetMaterialLibrary))))
              (:Finished
                (Variables|Default|SetIsRun? false)
                (Utilities|Array|SetArrayElem (Variables|Default|GetBuilding_LayeringState) (Variables|Default|GetNow_FloorNumber) "1"))))
          (:then_1
            (CallFunction|OnlyShowAreaActor _returnvalue_2)))))))

(event Custom|Set_Floor_Tag
  (bind _building_floor (Variables|Default|GetBuilding_Floor))
  ;[0 0 0] Event
  ;;[0 0 0] Set_Floor_Tag
  (Utilities|FlowControl|DoN (Variables|Default|GetNumberOfFloors) :!label _label
    (:Exit
      (bind _values (Utilities|Map|Values _building_floor))
      (bind _keys (Utilities|Map|Keys _building_floor))
      (Utilities|IsValid (Utilities|Array|Get(acopy) _values (Variables|Default|GetLocalVariables_1))
        (:Is%20Valid
          (Utilities|Array|Add (Variables|/Script/Engine.Actor|GetTags (Utilities|Array|Get(acopy) _values (Variables|Default|GetLocalVariables_1))) "SMBD")
          (Utilities|Array|Add (Variables|/Script/Engine.Actor|GetTags (Utilities|Array|Get(acopy) _values (Variables|Default|GetLocalVariables_1))) (Utilities|String|StringToName (Utilities|String|Append (CallFunction|DisplayNameCutNubmer (Utilities|GetDisplayName (Variables|Default|GetBuildingActor))) ":" (Utilities|Array|Get(acopy) _keys (Utilities|Array|FindItem _values (Utilities|Array|Get(acopy) _values (Variables|Default|GetLocalVariables_1)))))))
          (for _array_element (CallFunction|GetAllAttachedActors (Utilities|Array|Get(acopy) _values (Variables|Default|GetLocalVariables_1)))
            (Utilities|Array|Add (Variables|/Script/Engine.Actor|GetTags _array_element) "SMBD")
            (Utilities|Array|Add (Variables|/Script/Engine.Actor|GetTags _array_element) (Utilities|String|StringToName (Utilities|String|Append (CallFunction|DisplayNameCutNubmer (Utilities|GetDisplayName (Variables|Default|GetBuildingActor))) ":" (Utilities|Array|Get(acopy) _keys (Utilities|Array|FindItem _values (Utilities|Array|Get(acopy) _values (Variables|Default|GetLocalVariables_1))))))))
          (Math|Integer|IncrementInt (Variables|Default|GetLocalVariables_1)
            (:%20%20
              (goto _label))))
        (:Is%20Not%20Valid
          (goto _label))))))

(event Custom|HidetAllAreaActor
  ;[0 0 0] Event
  ;;[0 0 0] HidetAllAreaActor
  (Rendering|Material|SetScalarParameterValue "/Game/AssetLibrary/4_BPTools/SmartBuilding/Materials/MPC_Area.MPC_Area" "Area_Opacity" 0.0 :!class /Script/Engine.KismetMaterialLibrary)
  (bind _values (Utilities|Map|Values (Variables|Default|GetAreaActors)))
  (for _array_element _values
    (Transformation|SetActorScale3D _array_element "0, 0, 0")))

(event Custom|OnlyShowAreaActor
  (params (B :type String))
  ;[0 0 0] Event
  ;;[0 0 0] OnlyShowAreaActor
  (bind _keys (Utilities|Map|Keys (Variables|Default|GetAreaActors)))
  (for _array_element _keys
    (if (Utilities|Enum|Equal(Enum) _array_element (Utilities|String|Append B "_" "Area"))
      (Transformation|SetActorScale3D (.Value (Utilities|Map|Find (Variables|Default|GetAreaActors) _array_element)) "1.000000,1.000000,1.000000")
      (else
        (Transformation|SetActorScale3D (.Value (Utilities|Map|Find (Variables|Default|GetAreaActors) _array_element)) "0, 0, 0")))))

(event Custom|HideAreaActor
  (params (B :type String))
  ;[0 0 0] Event
  ;;[0 0 0] HideAreaActor
  (bind _keys (Utilities|Map|Keys (Variables|Default|GetAreaActors)))
  (for _array_element _keys
    (if (Utilities|Enum|Equal(Enum) _array_element (Utilities|String|Append B "_" "Area"))
      (Transformation|SetActorScale3D (.Value (Utilities|Map|Find (Variables|Default|GetAreaActors) _array_element)) "0, 0, 0"))))

(event Custom|GetBuildingTopFloor
  (bind _lowestfloor (Variables|Default|GetLowestFloor))
  ;[0 0 0] Event
  ;;[0 0 0] 注释
  (if (not (.ReturnValue (Utilities|Map|Find (Variables|Default|GetBuilding_Floor) "Roof")))
    (if (== (Variables|Default|GetLowestFloor) 1)
      (bind _values (Utilities|Map|Values (Variables|Default|GetBuilding_Floor)))
      (Variables|Default|SetTopFloor (Utilities|Array|Length _values))
      (elif (< _lowestfloor 1)
        (bind _values_2 (Utilities|Map|Values (Variables|Default|GetBuilding_Floor)))
        (Variables|Default|SetTopFloor (- (Utilities|Array|Length _values_2) (Math|Integer|Absolute(Integer) _lowestfloor)))))))

(event Custom|GetAreaActor
  ;[0 0 0] Event
  ;;[0 0 0] GetAreaActor
  (bind _values (Utilities|Map|Values (Variables|Default|GetBuilding_Floor)))
  (bind _counter (Utilities|FlowControl|DoN (Utilities|Array|Length _values) :!label _label)
    (:Exit
      (Utilities|IsValid (Utilities|Array|Get(acopy) _values (- _counter 1))
        (:Is%20Valid
          (for _array_element (Actor|GetAttachedActors (Utilities|Array|Get(acopy) _values (- _counter 1)) true false)
            (if (Utilities|Enum|Equal(Enum) (Utilities|Select :Index (Variables|Default|GetE_FloorBuildType) :NewEnumerator0 (Utilities|GetObjectName (Variables|/Script/Engine.Actor|GetRootComponent _array_element)) :NewEnumerator1 (CallFunction|DisplayNameCutNubmer (Utilities|GetDisplayName _array_element))) (Utilities|String|Append (Utilities|Select :Index (Variables|Default|GetE_FloorBuildType) :NewEnumerator0 (Utilities|GetObjectName (Variables|/Script/Engine.Actor|GetRootComponent (Utilities|Array|Get(acopy) _values (- _counter 1)))) :NewEnumerator1 (CallFunction|DisplayNameCutNubmer (Utilities|GetDisplayName (Utilities|Array|Get(acopy) _values (- _counter 1))))) "_" "Area"))
              (Utilities|Map|Add (Variables|Default|GetAreaActors) (Utilities|String|Append (Utilities|Select :Index (Variables|Default|GetE_FloorBuildType) :NewEnumerator0 (Utilities|GetObjectName (Variables|/Script/Engine.Actor|GetRootComponent (Utilities|Array|Get(acopy) _values (- _counter 1)))) :NewEnumerator1 (CallFunction|DisplayNameCutNubmer (Utilities|GetDisplayName (Utilities|Array|Get(acopy) _values (- _counter 1))))) "_" "Area") _array_element)))
          (goto _label))
        (:Is%20Not%20Valid
          (goto _label))))))

(event Custom|SetSMBDTag
  (bind _buildingactor (Variables|Default|GetBuildingActor))
  ;[0 0 0] Event
  ;;[0 0 0] AddSelfTag（给自身打标签）
  (Utilities|Array|Add (Variables|Actor|GetTags self) (Utilities|String|StringToName (Utilities|Select :Index (Variables|Default|GetE_FloorBuildType) :NewEnumerator0 (Utilities|GetObjectName (Variables|/Script/Engine.Actor|GetRootComponent _buildingactor)) :NewEnumerator1 (CallFunction|DisplayNameCutNubmer (Utilities|GetDisplayName _buildingactor))))))

(event Custom|GetFloorLocation_Layer
  (bind _floorlocation_layering (Variables|Default|GetFloorLocation_Layering))
  ;[0 0 0] Event
  ;;[0 0 0] GetFloorLocation_Layer
  (Utilities|Array|Clear _floorlocation_layering)
  (bind _values (Utilities|Map|Values (Variables|Default|GetBuilding_Floor)))
  (for _array_element _values
    (Utilities|Array|Add _floorlocation_layering (Transformation|GetActorLocation _array_element))))

(event Custom|GetFloorLocation_PullPush
  ;[0 0 0] Event
  ;;[0 0 0] GetFloorLocation_PullPush
  (Utilities|Map|Clear (Variables|Default|GetFloorLocation_PullPush))
  (bind _values (Utilities|Map|Values (Variables|Default|GetBuilding_Floor)))
  (for _array_element _values
    (Utilities|IsValid _array_element
      (:Is%20Valid
        (Development|PrintString (Utilities|String|Append (Utilities|Select :Index (Variables|Default|GetE_FloorBuildType) :NewEnumerator0 (Utilities|GetObjectName (Variables|/Script/Engine.Actor|GetRootComponent _array_element)) :NewEnumerator1 (CallFunction|DisplayNameCutNubmer (Utilities|GetDisplayName _array_element))) (Utilities|String|ToString(Vector) (Transformation|GetActorLocation _array_element))) false false)
        (Utilities|Map|Add (Variables|Default|GetFloorLocation_PullPush) (Utilities|Select :Index (Variables|Default|GetE_FloorBuildType) :NewEnumerator0 (Utilities|GetObjectName (Variables|/Script/Engine.Actor|GetRootComponent _array_element)) :NewEnumerator1 (CallFunction|DisplayNameCutNubmer (Utilities|GetDisplayName _array_element))) (Transformation|GetActorLocation _array_element))))))

(event Custom|BuildLayeringState
  ;[0 0 0] Event
  ;;[0 0 0] Building Layering State（创建楼层分层状态）
  (Utilities|Array|Clear (Variables|Default|GetBuilding_LayeringState))
  (bind _keys (Utilities|Map|Keys (Variables|Default|GetBuilding_Floor)))
  (for _array_element _keys
    (Utilities|Array|Add (Variables|Default|GetBuilding_LayeringState) "0")))

(event Custom|Get%20Underground%20Floor%20Height
  ;[0 0 0] Event
  ;;[0 0 0] Get Underground Floor Height
  (bind _values (Utilities|Map|Values (Variables|Default|GetBuilding_Floor)))
  (for _array_element _values
    (Utilities|IsValid _array_element
      (:Is%20Valid
        (if (== _array_element (.Value (Utilities|Map|Find (Variables|Default|GetBuilding_Floor) (Utilities|String|Append (Utilities|String|ToString(Integer) (Variables|Default|GetLowestFloor)) "F"))))
          (Variables|Default|SetUndergroundFloorHeight (Math|Float|Absolute(Float) (- (.z (Transformation|GetActorLocation _array_element)) (.z (Transformation|GetActorLocation (.Value (Utilities|Map|Find (Variables|Default|GetBuilding_Floor) "1F"))))))))))))

(event Custom|SMBD_%20Floor%20LayeringDisplay
  (bind _lowestfloor (Variables|Default|GetLowestFloor))
  (bind _returnvalue (Math|Integer|Absolute(Integer) _lowestfloor))
  ;[0 0 0] Building_Layering
  (if (not (Variables|Default|GetIsRun?))
    (if (not (Variables|Default|GetisBuildingLayering?))
      (Utilities|FlowControl|Sequence
        (:then_0
          (CallFunction|GetFloorLocationLayer))
        (:then_1
          (Variables|Default|SetIsRun? true)
          (bind _新建轨迹_0 (Timeline|时间轴_0 PlayFromStart)
            (:Update
              (bind _values (Utilities|Map|Values (Variables|Default|GetBuilding_Floor)))
              (for (_array_element _array_index) _values
                (Utilities|IsValid _array_element
                  (:Is%20Valid
                    (Transformation|SetActorLocation _array_element (Math|Vector|MakeVector (.x (Utilities|Array|Get(acopy) (Variables|Default|GetFloorLocation_Layering) _array_index)) (.y (Utilities|Array|Get(acopy) (Variables|Default|GetFloorLocation_Layering) _array_index)) (Math|Float|Lerp (.z (Utilities|Array|Get(acopy) (Variables|Default|GetFloorLocation_Layering) _array_index)) (+ (.z (Utilities|Array|Get(acopy) (Variables|Default|GetFloorLocation_Layering) _array_index)) (+ (+ (* (Variables|Default|GetLayeringHeight) (Math|Conversions|ToFloat(Integer) (select (Utilities|Enum|Equal(Enum) (Utilities|Select :Index (Variables|Default|GetE_FloorBuildType) :NewEnumerator0 (Utilities|GetObjectName (Variables|/Script/Engine.Actor|GetRootComponent _array_element)) :NewEnumerator1 (Utilities|GetDisplayName _array_element)) "Roof") (select (< (Variables|Default|GetLowestFloor) 0) (- (Utilities|Array|Length _values) 1) (Utilities|Array|Length _values)) (select (< (Math|Conversions|ToInteger(Byte) (Utilities|String|LeftChop (Utilities|Select :Index (Variables|Default|GetE_FloorBuildType) :NewEnumerator0 (Utilities|GetObjectName (Variables|/Script/Engine.Actor|GetRootComponent _array_element)) :NewEnumerator1 (Utilities|GetDisplayName _array_element)) 1)) 0) (+ (Math|Conversions|ToInteger(Byte) (Utilities|String|LeftChop (Utilities|Select :Index (Variables|Default|GetE_FloorBuildType) :NewEnumerator0 (Utilities|GetObjectName (Variables|/Script/Engine.Actor|GetRootComponent _array_element)) :NewEnumerator1 (Utilities|GetDisplayName _array_element)) 1)) _returnvalue) (+ (Math|Conversions|ToInteger(Byte) (Utilities|String|LeftChop (Utilities|Select :Index (Variables|Default|GetE_FloorBuildType) :NewEnumerator0 (Utilities|GetObjectName (Variables|/Script/Engine.Actor|GetRootComponent _array_element)) :NewEnumerator1 (Utilities|GetDisplayName _array_element)) 1)) (- _returnvalue 1)))))) (Variables|Default|GetUndergroundFloorHeight)) (Variables|Default|GetLayering_BaseHeight))) _新建轨迹_0)) false false)))))
            (:Finished
              (Variables|Default|SetIsRun? false)
              (Variables|Default|SetisBuildingLayering? true))))
        (:then_2
          (CallFunction|HidetAllAreaActor))))))

(event Custom|SMBD%20Floor%20NormalDisplay
  (bind _lowestfloor (Variables|Default|GetLowestFloor))
  (bind _returnvalue (Math|Integer|Absolute(Integer) _lowestfloor))
  ;[0 0 0] Building_BackToNormal
  (if (Variables|Default|GetisBuildingLayering?)
    (if (not (Variables|Default|GetIsRun?))
      (for (_array_element _array_index) (Variables|Default|GetBuilding_LayeringState)
        (if (Utilities|Enum|Equal(Enum) _array_element "1")
          (CallFunction|ResetLayering _array_index)))
      (Variables|Default|SetIsRun? true)
      (Utilities|FlowControl|Sequence
        (:then_0
          (CallFunction|GetFloorLocationLayer))
        (:then_1
          (bind _新建轨迹_0 (Timeline|时间轴_1 PlayFromStart)
            (:Update
              (bind _values (Utilities|Map|Values (Variables|Default|GetBuilding_Floor)))
              (for (_array_element_2 _array_index_2) _values
                (Utilities|IsValid _array_element_2
                  (:Is%20Valid
                    (Transformation|SetActorLocation _array_element_2 (Math|Vector|MakeVector (.x (Utilities|Array|Get(acopy) (Variables|Default|GetFloorLocation_Layering) _array_index_2)) (.y (Utilities|Array|Get(acopy) (Variables|Default|GetFloorLocation_Layering) _array_index_2)) (Math|Float|Lerp (.z (Utilities|Array|Get(acopy) (Variables|Default|GetFloorLocation_Layering) _array_index_2)) (- (.z (Utilities|Array|Get(acopy) (Variables|Default|GetFloorLocation_Layering) _array_index_2)) (+ (+ (* (Variables|Default|GetLayeringHeight) (Math|Conversions|ToFloat(Integer) (select (Utilities|Enum|Equal(Enum) (Utilities|Select :Index (Variables|Default|GetE_FloorBuildType) :NewEnumerator0 (Utilities|GetObjectName (Variables|/Script/Engine.Actor|GetRootComponent _array_element_2)) :NewEnumerator1 (Utilities|GetDisplayName _array_element_2)) "Roof") (select (< (Variables|Default|GetLowestFloor) 0) (- (Utilities|Array|Length _values) 1) (Utilities|Array|Length _values)) (select (< (Math|Conversions|ToInteger(Byte) (Utilities|String|LeftChop (Utilities|Select :Index (Variables|Default|GetE_FloorBuildType) :NewEnumerator0 (Utilities|GetObjectName (Variables|/Script/Engine.Actor|GetRootComponent _array_element_2)) :NewEnumerator1 (Utilities|GetDisplayName _array_element_2)) 1)) 0) (+ (Math|Conversions|ToInteger(Byte) (Utilities|String|LeftChop (Utilities|Select :Index (Variables|Default|GetE_FloorBuildType) :NewEnumerator0 (Utilities|GetObjectName (Variables|/Script/Engine.Actor|GetRootComponent _array_element_2)) :NewEnumerator1 (Utilities|GetDisplayName _array_element_2)) 1)) _returnvalue) (+ (Math|Conversions|ToInteger(Byte) (Utilities|String|LeftChop (Utilities|Select :Index (Variables|Default|GetE_FloorBuildType) :NewEnumerator0 (Utilities|GetObjectName (Variables|/Script/Engine.Actor|GetRootComponent _array_element_2)) :NewEnumerator1 (Utilities|GetDisplayName _array_element_2)) 1)) (- _returnvalue 1)))))) (Variables|Default|GetUndergroundFloorHeight)) (Variables|Default|GetLayering_BaseHeight))) _新建轨迹_0)) false false)))))
            (:Finished
              (Variables|Default|SetIsRun? false)
              (Variables|Default|SetisBuildingLayering? false))))
        (:then_2
          (CallFunction|HidetAllAreaActor))))))

(event EventBeginPlay
  ;[0 0 0] BeginPlay
  (Utilities|FlowControl|Sequence
    (:then_0
      ;;[0 0 0] ShowMouse（显示鼠标）
      (Variables|/Script/Engine.PlayerController|SetbShowMouseCursor (Game|GetPlayerController 0) true))
    (:then_1
      ;;[0 0 0] Get Number Of Floors（获取楼层数）
      (bind _values (Utilities|Map|Values (Variables|Default|GetBuilding_Floor)))
      (Variables|Default|SetNumberOfFloors (Utilities|Array|Length _values)))
    (:then_2
      (CallFunction|BuildLayeringState) ; 创建楼层分层状态
    )
    (:then_3
      (CallFunction|SetFloorTag) ; 给每个楼层及每个楼层下的模型打标签
    )
    (:then_4
      (CallFunction|GetUndergroundFloorHeight) ; 获取地下层至1层的高度差
    )
    (:then_5
      (CallFunction|GetFloorLocationPullPush) ; 获取楼层的抽拉坐标
    )
    (:then_6)
    (:then_7
      (CallFunction|HidetAllAreaActor) ; 隐藏所有区域模型
    )
    (:then_8
      (CallFunction|GetBuildingTopFloor))
    (:then_9
      (CallFunction|SetSMBDTag))))

(fn ConstructionScript)

(fn APISMBDFloorLayeringDisplay
  (CallFunction|SMBDFloorLayeringDisplay))

(fn APISMBDFloorBacktoNormalDisplay
  (CallFunction|SMBDFloorNormalDisplay))

(fn APISMBDFloorPull
  (params (NumberOfFloor :type Integer))
  (CallFunction|SMBDFloorPull NumberOfFloor))

(fn APISMBDFloorPush
  (params (NumberOfFloor :type Integer))
  (CallFunction|SMBDFloorPush NumberOfFloor))

(fn APISMBDFloorHide
  (params (NumberOfFloors :type Array%20of%20Integers))
  (for _array_element NumberOfFloors
    (Transformation|SetActorScale3D (.Value (Utilities|Map|Find (Variables|Default|GetBuilding_Floor) (Utilities|String|Append (Utilities|String|ToString(Integer) _array_element) "F"))) "0, 0, 0")))

(fn APISMBDFloorHideAboveFloor
  (params (NumberOfFloor :type Integer))
  (bind _building_floor (Variables|Default|GetBuilding_Floor))
  (bind _values (Utilities|Map|Values _building_floor))
  (Utilities|Map|Keys _building_floor)
  (for _array_element _values
    (if (== (Math|Conversions|ToInteger(Byte) (Utilities|String|LeftChop (Utilities|GetObjectName _array_element) 1)) 0)
      (Transformation|SetActorScale3D _array_element "0, 0, 0")
      (elif (<= (Math|Conversions|ToInteger(Byte) (Utilities|String|LeftChop (Utilities|GetObjectName _array_element) 1)) NumberOfFloor)
        (Transformation|SetActorScale3D _array_element "1.000000,1.000000,1.000000")
        (elif (> (Math|Conversions|ToInteger(Byte) (Utilities|String|LeftChop (Utilities|GetObjectName _array_element) 1)) NumberOfFloor)
          (Transformation|SetActorScale3D _array_element "0, 0, 0"))))))

(fn APISMBDFloorHideAll
  (bind _values (Utilities|Map|Values (Variables|Default|GetBuilding_Floor)))
  (for _array_element _values
    (Transformation|SetActorScale3D _array_element "0, 0, 0")))

(fn APISMBDFloorShow
  (params (NumberOfFloors :type Array%20of%20Integers))
  (for _array_element NumberOfFloors
    (Transformation|SetActorScale3D (.Value (Utilities|Map|Find (Variables|Default|GetBuilding_Floor) (Utilities|String|Append (Utilities|String|ToString(Integer) _array_element) "F"))) "1.000000,1.000000,1.000000")))

(fn APISMBDFloorShowAll
  (bind _values (Utilities|Map|Values (Variables|Default|GetBuilding_Floor)))
  (for _array_element _values
    (Transformation|SetActorScale3D _array_element "1.000000,1.000000,1.000000")))

(fn GetAllAttachedActors
  (params (RootActor :type Actor%20Object%20Reference))
  (bind _result (LocalVariables|GetResult))
  (CallFunction|GetAllAttachedActorsInternal RootActor _result)
  (return _result))

(fn GetAllAttachedActorsInternal
  (params (RootActor :type Actor%20Object%20Reference) (Result :type Array%20of%20Actor%20Object%20References))
  (for _array_element (Actor|GetAttachedActors RootActor true false)
    (Utilities|FlowControl|Sequence
      (:then_0
        (Utilities|Array|Add Result _array_element))
      (:then_1
        (CallFunction|GetAllAttachedActorsInternal _array_element Result)))))