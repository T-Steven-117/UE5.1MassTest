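; Clickable actor, apparently a stacked model, that toggles the vertical layout of its chained components.
; BeginPlay recursively collects each first child from the root into CompRef and binds OnClicked on its static meshes.
; Clicking a non-root component flip-flops between lifting each component 30 units and spacing each 100 units above the previous, aligned in X/Y.
; An OnRep-triggered RPC event reuses that logic, but the IsRPC toggle is unwired.
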(event Custom|CustomEvent
  (params (TouchedComponent :type Primitive%20Component%20Object%20Reference) (ButtonPressed :type Key%20Structure :default "None"))
  (for (_array_element _array_index) (Variables|Default|GetCompRef)
    (if (!= _array_index 0)
      (if (Utilities|Enum|Equal(Enum) (Utilities|GetDisplayName _array_element) (Utilities|GetDisplayName TouchedComponent))
        (Utilities|FlowControl|FlipFlop
          (:A
            (for (_array_element_2 _array_index_2) (Variables|Default|GetCompRef)
              (if (!= _array_index_2 0)
                (Transformation|SetWorldLocation _array_element_2 (Math|Vector|MakeVector (.x (Transformation|GetWorldLocation (Variables|Default|GetArray%20Element))) (.y (Transformation|GetWorldLocation (Variables|Default|GetArray%20Element))) (+ (.z (Transformation|GetWorldLocation (Variables|Default|GetArray%20Element))) (+ (- (.z (Transformation|GetWorldLocation _array_element_2)) (.z (Transformation|GetWorldLocation (Variables|Default|GetArray%20Element)))) 3e+01))) false false))
              (Variables|Default|SetArray%20Element _array_element_2))
            (Variables|Default|SetArray%20Element 0))
          (:B
            (for (_array_element_3 _array_index_3) (Variables|Default|GetCompRef)
              (if (!= _array_index_3 0)
                (Transformation|SetWorldLocation _array_element_3 (Math|Vector|MakeVector (.x (Transformation|GetWorldLocation (Variables|Default|GetArray%20Element))) (.y (Transformation|GetWorldLocation (Variables|Default|GetArray%20Element))) (+ (.z (Transformation|GetWorldLocation (Variables|Default|GetArray%20Element))) 1e+02)) false false))
              (Variables|Default|SetArray%20Element _array_element_3))
            (Variables|Default|SetArray%20Element 0)))))))

(event Custom|RPC
  (params (TouchedComponent :type Primitive%20Component%20Object%20Reference) (ButtonPressed :type Key%20Structure :default "None"))
  (for (_array_element _array_index) (Variables|Default|GetCompRef)
    (if (!= _array_index 0)
      (if (Utilities|Enum|Equal(Enum) (Utilities|GetDisplayName _array_element) (Utilities|GetDisplayName (stale Custom|CustomEvent TouchedComponent)))
        (Utilities|FlowControl|FlipFlop
          (:A
            (for (_array_element_2 _array_index_2) (Variables|Default|GetCompRef)
              (if (!= _array_index_2 0)
                (Transformation|SetWorldLocation _array_element_2 (Math|Vector|MakeVector (.x (Transformation|GetWorldLocation (Variables|Default|GetArray%20Element))) (.y (Transformation|GetWorldLocation (Variables|Default|GetArray%20Element))) (+ (.z (Transformation|GetWorldLocation (Variables|Default|GetArray%20Element))) (+ (- (.z (Transformation|GetWorldLocation _array_element_2)) (.z (Transformation|GetWorldLocation (Variables|Default|GetArray%20Element)))) 3e+01))) false false))
              (Variables|Default|SetArray%20Element _array_element_2))
            (Variables|Default|SetArray%20Element 0))
          (:B
            (for (_array_element_3 _array_index_3) (Variables|Default|GetCompRef)
              (if (!= _array_index_3 0)
                (Transformation|SetWorldLocation _array_element_3 (Math|Vector|MakeVector (.x (Transformation|GetWorldLocation (Variables|Default|GetArray%20Element))) (.y (Transformation|GetWorldLocation (Variables|Default|GetArray%20Element))) (+ (.z (Transformation|GetWorldLocation (Variables|Default|GetArray%20Element))) 1e+02)) false false))
              (Variables|Default|SetArray%20Element _array_element_3))
            (Variables|Default|SetArray%20Element 0)))))))

(event EventBeginPlay
  (bind _rootcomponent (Variables|Transformation|GetRootComponent))
  (Utilities|Array|AddUnique (Variables|Default|GetCompRef) _rootcomponent)
  (bind _children (CallFunction|GetAll _rootcomponent))
  (for _array_element _children
    (bind _asstatic_mesh_component (Utilities|Casting|CastToStaticMeshComponent _array_element))
    (EventDispatchers|BindEventtoOnClicked _asstatic_mesh_component (delegate Custom|CustomEvent))))

(fn ConstructionScript)

(fn GetAll
  (params (Target :type Scene%20Component%20Object%20Reference))
  (bind _returnvalue (Components|GetChildComponent Target 0))
  (bind _compref (Variables|Default|GetCompRef))
  (Utilities|IsValid _returnvalue
    (:Is%20Valid
      (Utilities|Array|AddUnique _compref _returnvalue)
      (CallFunction|GetAll _returnvalue)
      (return _compref))
    (:Is%20Not%20Valid
      (return _compref))))

(fn OnRepBIsRPC
  (if (Variables|Default|GetbIsRPC)
    (CallFunction|RPC (Variables|Default|GetTouched%20Component) "None")))